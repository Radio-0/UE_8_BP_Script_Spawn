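; Player paddle pawn for what appears to be a ball-and-lives game, spawning and tracking a BP_Sphere ball.
; MoveRight input slides it along Y in fixed, swept steps that are not scaled by axis magnitude or frame time.
; On BeginPlay, if lives remain, it decrements LifeNumber and calls SpawnBall, which spawns the ball at the capsule and binds to its OnDead event.
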(event EventBeginPlay
  (if (!= (Variables|Default|GetLifeNumber) 0)
    (bind _result (Math|Integer|DecrementInt (Variables|Default|GetLifeNumber))
      (:%20%20
        (CallFunction|SpawnBall)
        (Variables|Default|SetLifeNumber _result)))))

(event Collision|EventActorBeginOverlap
  (params (OtherActor :type Actor%20Object%20Reference))
  (Transformation|AddActorWorldOffset "0, 0, 0" true))

(event EventTick
  (params (DeltaSeconds :type Float%20%28single-precision%29)))

(event Input|AxisEvents|InputAxisMoveRight
  (params (AxisValue :type Float%20%28single-precision%29))
  (if (< AxisValue 0.0)
    (bind _sweephitresult (Transformation|AddActorWorldOffset "0,-50.000000, 0" true))
    (if (.bBlockingHit (Collision|BreakHitResult _sweephitresult))
      _)))

(event Input|AxisEvents|InputAxisMoveRight
  (params (AxisValue :type Float%20%28single-precision%29))
  (if (> AxisValue 0.0)
    (bind _sweephitresult (Transformation|AddActorWorldOffset "0,50.000000, 0" true))
    (if (.bBlockingHit (Collision|BreakHitResult _sweephitresult))
      _)))

(fn ConstructionScript)

(fn SpawnBall
  (bind _returnvalue (Game|SpawnActorfromClass "/Game/BP_Sphere.BP_Sphere_C" (Math|Transform|MakeTransform (Transformation|GetWorldLocation (Variables|Default|GetCapsule)) "0, 0, 0" "1,1,1") "AlwaysSpawn" 0 0))
  (bind _output_get (Variables|Default|SetPlayingBall _returnvalue))
  (EventDispatchers|BindEventtoOnDead _output_get (EventDispatchers|CreateEvent :!event SpawnBall))
  (return))